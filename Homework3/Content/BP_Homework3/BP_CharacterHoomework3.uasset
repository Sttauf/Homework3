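; Player character Blueprint handling mouse look, WASD movement, crouch, prone, sprint and aiming.
; Input events set state flags that gate movement and choose standing or crouched aim montages.
; Sprint raises walk speed and opens a Gate so Tick drives forward movement along control yaw, replacing WASD until release or crouch.
; Prone blocks movement, and releasing it clears InputEnable, which this graph never sets back.
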(event EventTick
  (params (DeltaSeconds :type Float%20%28single-precision%29))
  ;[1 1 1] Shift
  (if (and (Variables|Default|GetSprintPressed) (Variables|Default|GetCrouchPressed))
    (Variables|Default|SetSprintPressed false)
    (Variables|/Script/Engine.CharacterMovementComponent|SetMaxWalkSpeed (Variables|Character|GetCharacterMovement) 5e+02)
    (goto _label Close)
    (elif (Variables|Default|GetInputEnable)
      (Utilities|FlowControl|Gate true :!label _label ; When pressing the Shift, I allow (Open) Event Tick\nto have access to add movement, when I release \nShift, I block (Close) Event Tick to have access to\nadd movement.
        (:Exit
          (Pawn|Input|AddMovementInput (Math|Vector|GetForwardVector (Math|Rotator|MakeRotator 0.0 0.0 (.yaw (Pawn|GetControlRotation :!class /Script/Engine.Pawn)))) 1e+04 false))))))

(event Input|ActionEvents|InputActionSprint
  (params (Key :type Key%20Structure))
  (bind _charactermovement (Variables|Character|GetCharacterMovement))
  (bind _pronepressed (Variables|Default|GetPronePressed))
  ;[1 1 1] Shift
  (:Pressed
    (if (not _pronepressed)
      (Variables|Default|SetSprintPressed true)
      (Variables|/Script/Engine.CharacterMovementComponent|SetMaxWalkSpeed _charactermovement 7.5e+02)
      (Utilities|FlowControl|Gate true) ; enters at Open
    ))
  (:Released
    (if (not _pronepressed)
      (Variables|Default|SetSprintPressed false)
      (Variables|/Script/Engine.CharacterMovementComponent|SetMaxWalkSpeed _charactermovement 5e+02)
      (Utilities|FlowControl|Gate true) ; enters at Close
    )))

(event Input|ActionEvents|InputActionProne
  (params (Key :type Key%20Structure))
  ;[1 1 1] C
  (:Pressed
    (Variables|Default|SetPronePressed true))
  (:Released
    (Variables|Default|SetPronePressed false)
    (Variables|Default|SetInputEnable false)))

(event Input|AxisEvents|InputAxisTurn
  (params (AxisValue :type Float%20%28single-precision%29))
  ;[1 1 1] Mouse Position/Camera Rotation
  (Pawn|Input|AddControllerYawInput AxisValue) ; Zaxis
)

(event Input|AxisEvents|InputAxisLookUp
  (params (AxisValue :type Float%20%28single-precision%29))
  ;[1 1 1] Mouse Position/Camera Rotation
  (Pawn|Input|AddControllerPitchInput AxisValue) ; Xaxis
)

(event Input|AxisEvents|InputAxisMoveForward
  (params (AxisValue :type Float%20%28single-precision%29))
  (bind _returnvalue (Pawn|GetControlRotation :!class /Script/Engine.Pawn))
  (bind _returnvalue_2 (Math|Rotator|MakeRotator 0.0 0.0 (.yaw _returnvalue)))
  (bind _returnvalue_3 (Math|Vector|GetForwardVector _returnvalue_2))
  ;[1 1 1] Movement WASD
  (if (Variables|Default|GetInputEnable) ; INPUT
    (if (not (Variables|Default|GetPronePressed)) ; PRONE
      (if (Variables|Default|GetCrouchPressed) ; CROUCH
        (Pawn|Input|AddMovementInput _returnvalue_3 AxisValue false) ; W/S CROUCH
        (elif (not (Variables|Default|GetSprintPressed)) ; SPRINT
          (Pawn|Input|AddMovementInput _returnvalue_3 AxisValue false) ; W/S WALK
        )))))

(event Input|AxisEvents|InputAxisMoveRight
  (params (AxisValue :type Float%20%28single-precision%29))
  (bind _returnvalue (Pawn|GetControlRotation :!class /Script/Engine.Pawn))
  (bind _returnvalue_2 (Math|Rotator|MakeRotator 0.0 0.0 (.yaw _returnvalue)))
  (bind _returnvalue_3 (Math|Vector|GetRightVector _returnvalue_2))
  ;[1 1 1] Movement WASD
  (if (Variables|Default|GetInputEnable) ; INPUT
    (if (not (Variables|Default|GetPronePressed)) ; PRONE
      (if (Variables|Default|GetCrouchPressed) ; CROUCH
        (Pawn|Input|AddMovementInput _returnvalue_3 AxisValue false) ; A/D CROUCH
        (elif (not (Variables|Default|GetSprintPressed)) ; SPRINT
          (Pawn|Input|AddMovementInput _returnvalue_3 AxisValue false) ; A/D WALK
        )))))

(event Input|KeyboardEvents|LeftCtrl
  (params (Key :type Key%20Structure))
  (bind _mesh (Variables|Character|GetMesh))
  ;[1 1 1] Ctrl
  (:Pressed
    (Character|Crouch)
    (Variables|Default|SetCrouchPressed true)
    ;[1 1 1] RMouse
    (if (Variables|Default|GetRMousePressed)
      (Animation|Montage|PlayMontage _mesh "/Game/BP_Homework3/AM_AimCrouch.AM_AimCrouch")))
  (:Released
    (Character|UnCrouch)
    (Variables|Default|SetCrouchPressed false)
    (if (Variables|Default|GetRMousePressed)
      (Animation|Montage|PlayMontage _mesh "/Game/BP_Homework3/AM_Aim.AM_Aim"))))

(event Input|MouseEvents|RightMouseButton
  (params (Key :type Key%20Structure))
  (bind _mesh (Variables|Character|GetMesh))
  (bind _crouchpressed (Variables|Default|GetCrouchPressed))
  ;[1 1 1] RMouse
  (:Pressed
    (if (not (Variables|Default|GetSprintPressed))
      (if (not (Variables|Default|GetPronePressed))
        (Variables|Default|SetRMousePressed true)
        (if _crouchpressed
          (Animation|Montage|PlayMontage _mesh "/Game/BP_Homework3/AM_AimCrouch.AM_AimCrouch")
          (else
            (Animation|Montage|PlayMontage _mesh "/Game/BP_Homework3/AM_Aim.AM_Aim"))))))
  (:Released
    (Variables|Default|SetRMousePressed false)
    (if _crouchpressed
      (Animation|StopAnimMontage "/Game/BP_Homework3/AM_AimCrouch.AM_AimCrouch")
      (else
        (Animation|StopAnimMontage "/Game/BP_Homework3/AM_Aim.AM_Aim")))))

(fn ConstructionScript)